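; BP_LayComponent is a component that manages a character's lying-down state, lay type (back, belly, side) and pose for animation.
; Lay/Stand toggles standing and laying; inside a bed volume it snaps the character to the bed transform with gravity and collision off, restoring them on standing.
; Changing type while laying selects a roll and moves to Sitting.
; An InTransition flag blocks new requests during state, type or pose changes.
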(event `ChangeLayType`
  (params (NewParam :type "/Game/AnimationEducation/LLSS/AnimPacks/Lay/Blueprints/Enum/Enum_Faceing Enum" :default "NewEnumerator0"))
  (bind _laytype (`self.LayType`))
  ;[1 1 1 1 30] Comment
  (if (not (`self.InTransition`))
    (set `self.PreviousLayType` _laytype)
    (set `self.PreviousPose` 0)
    (switch `/Game/AnimationEducation/LLSS/AnimPacks/Lay/Blueprints/Enum/Enum_MainState` (`self.MainState`)
      (:`NewEnumerator0`
        (set `self.LayType` NewParam))
      (:`NewEnumerator1`
        (set `self.InTransition` true)
        (switch `/Game/AnimationEducation/LLSS/AnimPacks/Lay/Blueprints/Enum/Enum_Faceing` _laytype
          (:`NewEnumerator0`
            (bind _output_get (set `self.LayType` NewParam))
            (switch `/Game/AnimationEducation/LLSS/AnimPacks/Lay/Blueprints/Enum/Enum_Faceing` _output_get
              (:`NewEnumerator0`
                (set `self.MainState` "NewEnumerator1")
                (set `self.InTransition` false :!label _label))
              (:`NewEnumerator1`
                (set `self.RollType` "NewEnumerator0")
                (set `self.MainState` "NewEnumerator4" :!label _label_2))
              (:`NewEnumerator2`
                (set `self.RollType` "NewEnumerator4")
                (goto _label_2))))
          (:`NewEnumerator1`
            (bind _output_get_2 (set `self.LayType` NewParam))
            (switch `/Game/AnimationEducation/LLSS/AnimPacks/Lay/Blueprints/Enum/Enum_Faceing` _output_get_2
              (:`NewEnumerator0`
                (set `self.RollType` "NewEnumerator1")
                (goto _label_2))
              (:`NewEnumerator1`
                (set `self.MainState` "NewEnumerator1")
                (goto _label))
              (:`NewEnumerator2`
                (set `self.RollType` "NewEnumerator5")
                (goto _label_2))))
          (:`NewEnumerator2`
            (bind _output_get_3 (set `self.LayType` NewParam))
            (switch `/Game/AnimationEducation/LLSS/AnimPacks/Lay/Blueprints/Enum/Enum_Faceing` _output_get_3
              (:`NewEnumerator0`
                (set `self.RollType` "NewEnumerator2")
                (goto _label_2))
              (:`NewEnumerator1`
                (set `self.RollType` "NewEnumerator6")
                (goto _label_2))
              (:`NewEnumerator2`
                (set `self.MainState` "NewEnumerator1")
                (goto _label)))))))))

(event `Lay/Stand`
  (params (Character :type "Character Object Reference") (CharacterMovment :type "CharacterMovementComponent Object Reference"))
  (bind _capsulecomponent (`Character.CapsuleComponent` Character))
  ;[1 1 1 1 30] Comment
  (if (not (`self.InTransition`))
    (switch `/Game/AnimationEducation/LLSS/AnimPacks/Lay/Blueprints/Enum/Enum_MainState` (`self.MainState`)
      (:`NewEnumerator0`
        (set `self.MainState` "NewEnumerator1")
        (if (`self.InBedVolume`)
          (set `self.PreviousGravity` (`CharacterMovementComponent.GravityScale` CharacterMovment))
          (set `CharacterMovementComponent.GravityScale` 0.0 CharacterMovment)
          (`CharacterMovementComponent.SetMovementMode` CharacterMovment "MOVE_Flying" 0)
          (`NavMovementComponent.StopActiveMovement` CharacterMovment)
          (`PrimitiveComponent.SetCollisionEnabled` _capsulecomponent "NoCollision")
          (`Actor.K2_SetActorTransform` Character (`self.BedTransforms`) false false)
          (set `self.Forward` true)))
      (:`NewEnumerator1`
        (set `self.MainState` "NewEnumerator0")
        (`PrimitiveComponent.SetCollisionEnabled` (`Character.CapsuleComponent` Character) "QueryAndPhysics")
        (set `CharacterMovementComponent.GravityScale` (`self.PreviousGravity`) CharacterMovment)
        (`CharacterMovementComponent.SetMovementMode` CharacterMovment "MOVE_Walking" 0)
        (`PrimitiveComponent.SetCollisionEnabled` _capsulecomponent "QueryAndPhysics")))
    (set `self.InTransition` true)
    (set `self.PreviousPose` (`self.PoseNumber`))))

(event `ChangePose`
  (params (PoseNumber :type Integer))
  (if (and (!= PoseNumber (`self.PreviousPose`)) (not (`self.InTransition`)))
    (set `self.PoseNumber` PoseNumber)
    (set `self.InTransition` true)))