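; BP_LeanWall is a wall volume that marks a spot where characters with a BP_LLSS_Comp component can lean.
; On trigger overlap, if that component is not in transition and is in the required pose type, it receives the wall, lean type and target transform, with yaw offset by lean type.
; Leaving the trigger clears the component's in-volume flag.
; The construction script shows a pose number label when ForcedPose is set.
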(event `self.Trigger.OnComponentBeginOverlap`
  (params (OverlappedComponent :type "PrimitiveComponent Object Reference") (OtherActor :type "Actor Object Reference") (OtherComp :type "PrimitiveComponent Object Reference") (OtherBodyIndex :type Integer) (bFromSweep :type Boolean) (SweepResult :type "HitResult Structure (by ref)"))
  (bind _returnvalue (`SceneComponent.K2_GetComponentToWorld` (`self.Traget`)))
  (bind _ascharacter (cast `Character` OtherActor))
  (bind _returnvalue_2 (`self.GetComponentByClass` _ascharacter "/Game/AnimationEducation/LLSS/Blueprints/BP_LLSS_Comp.BP_LLSS_Comp_C"))
  (`/Engine/EditorBlueprintResources/StandardMacros.IsValid` _returnvalue_2
    (:`Is Valid`
      (if (and (not (`/Game/AnimationEducation/LLSS/Blueprints/BP_LLSS_Comp.InTransition` _returnvalue_2)) (`|EnumEquality` (`/Game/AnimationEducation/LLSS/Blueprints/BP_LLSS_Comp.PoseType` _returnvalue_2) "NewEnumerator0"))
        (bind _output_get (set `/Game/AnimationEducation/LLSS/Blueprints/BP_LLSS_Comp.LayType` (`self.LeanType`) _returnvalue_2))
        (set `/Game/AnimationEducation/LLSS/Blueprints/BP_LLSS_Comp.Mirror` false _returnvalue_2)
        (set `/Game/AnimationEducation/LLSS/Blueprints/BP_LLSS_Comp.ObjectTransforms` (`KismetMathLibrary.MakeTransform` (.location _returnvalue) (`KismetMathLibrary.MakeRotator` (.roll (.rotation _returnvalue)) (.pitch (.rotation _returnvalue)) (+ (.yaw (.rotation _returnvalue)) (select `/Game/AnimationEducation/LLSS/AnimPacks/Lay/Blueprints/Enum/Enum_Faceing` _output_get :`NewEnumerator0` 180.0 :`NewEnumerator2` 90.0)))) _returnvalue_2)
        (set `/Game/AnimationEducation/LLSS/Blueprints/BP_LLSS_Comp.InVolume` true _returnvalue_2)
        (set `/Game/AnimationEducation/LLSS/Blueprints/BP_LLSS_Comp.OverlappedChair` null _returnvalue_2)
        (set `/Game/AnimationEducation/LLSS/Blueprints/BP_LLSS_Comp.OverlappedBed` null _returnvalue_2)
        (set `/Game/AnimationEducation/LLSS/Blueprints/BP_LLSS_Comp.OverlappedWall` self _returnvalue_2)
        (set `/Game/AnimationEducation/LLSS/Blueprints/BP_LLSS_Comp.VolumeType` "NewEnumerator2" _returnvalue_2)))))

(event `self.Trigger.OnComponentEndOverlap`
  (params (OverlappedComponent :type "PrimitiveComponent Object Reference") (OtherActor :type "Actor Object Reference") (OtherComp :type "PrimitiveComponent Object Reference") (OtherBodyIndex :type Integer))
  (bind _ascharacter (cast `Character` OtherActor))
  (bind _returnvalue (`self.GetComponentByClass` _ascharacter "/Game/AnimationEducation/LLSS/Blueprints/BP_LLSS_Comp.BP_LLSS_Comp_C"))
  (`/Engine/EditorBlueprintResources/StandardMacros.IsValid` _returnvalue
    (:`Is Valid`
      (set `/Game/AnimationEducation/LLSS/Blueprints/BP_LLSS_Comp.InVolume` false _returnvalue))))

(fn `UserConstructionScript`
  (bind _textrender (`self.TextRender`))
  (`SceneComponent.SetVisibility` _textrender (`self.ForcedPose`) false)
  (`TextRenderComponent.K2_SetText` _textrender (`KismetTextLibrary.Conv_StringToText` (`KismetStringLibrary.Concat_StrStr` "" " No " (`KismetStringLibrary.Conv_IntToString` (`self.PoseNo`))))))