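; Bed actor that sets up a character's BP_LLSS_Comp for lying on a bed or on the ground.
; Left and right triggers, unless the component is mid-transition or in a blocking state, pass it the bed, mirror flag and yaw-offset target transform; exiting clears InVolume.
; ForcedPose overrides the lay type and clears chair and wall references.
; The construction script applies the mesh and shows a pose label when forced.
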(event `self.TriggerRight.OnComponentBeginOverlap`
  (params (OverlappedComponent :type "PrimitiveComponent Object Reference") (OtherActor :type "Actor Object Reference") (OtherComp :type "PrimitiveComponent Object Reference") (OtherBodyIndex :type Integer) (bFromSweep :type Boolean) (SweepResult :type "HitResult Structure (by ref)"))
  (bind _returnvalue (`SceneComponent.K2_GetComponentToWorld` (`self.RightTraget`)))
  (bind _ascharacter (cast `Character` OtherActor))
  (bind _returnvalue_2 (`self.GetComponentByClass` _ascharacter "/Game/AnimationEducation/LLSS/Blueprints/BP_LLSS_Comp.BP_LLSS_Comp_C"))
  (`/Engine/EditorBlueprintResources/StandardMacros.IsValid` _returnvalue_2
    (:`Is Valid`
      (set `/Game/AnimationEducation/LLSS/Blueprints/BP_LLSS_Comp.VolumeType` "NewEnumerator1" _returnvalue_2)
      (if (and (not (`/Game/AnimationEducation/LLSS/Blueprints/BP_LLSS_Comp.InTransition` _returnvalue_2)) (`|EnumInequality` (`/Game/AnimationEducation/LLSS/Blueprints/BP_LLSS_Comp.MainState` _returnvalue_2) "NewEnumerator1"))
        (bind _output_get (set `/Game/AnimationEducation/LLSS/Blueprints/BP_LLSS_Comp.BedGround` (`self.GroudBed`) _returnvalue_2))
        (set `/Game/AnimationEducation/LLSS/Blueprints/BP_LLSS_Comp.Mirror` false _returnvalue_2)
        (set `/Game/AnimationEducation/LLSS/Blueprints/BP_LLSS_Comp.ObjectTransforms` (`KismetMathLibrary.MakeTransform` (.location _returnvalue) (`KismetMathLibrary.MakeRotator` (.roll (.rotation _returnvalue)) (.pitch (.rotation _returnvalue)) (+ (.yaw (.rotation _returnvalue)) (select `/Game/AnimationEducation/LLSS/AnimPacks/Lay/Blueprints/Enum/Enum_BedGround` _output_get :`NewEnumerator0` -90.0 :`NewEnumerator1` 180.0)))) _returnvalue_2)
        (set `/Game/AnimationEducation/LLSS/Blueprints/BP_LLSS_Comp.InVolume` true _returnvalue_2)
        (set `/Game/AnimationEducation/LLSS/Blueprints/BP_LLSS_Comp.OverlappedBed` self _returnvalue_2)
        (if (`self.ForcedPose`)
          (bind _output_get_2 (set `/Game/AnimationEducation/LLSS/Blueprints/BP_LLSS_Comp.NextLayType` (`self.LayPose`) _returnvalue_2))
          (set `/Game/AnimationEducation/LLSS/Blueprints/BP_LLSS_Comp.LayType` _output_get_2 _returnvalue_2)
          (set `/Game/AnimationEducation/LLSS/Blueprints/BP_LLSS_Comp.OverlappedChair` null _returnvalue_2)
          (set `/Game/AnimationEducation/LLSS/Blueprints/BP_LLSS_Comp.OverlappedWall` null _returnvalue_2)
          (set `/Game/AnimationEducation/LLSS/Blueprints/BP_LLSS_Comp.VolumeType` "NewEnumerator1" _returnvalue_2))))))

(event `self.TriggerRight.OnComponentEndOverlap`
  (params (OverlappedComponent :type "PrimitiveComponent Object Reference") (OtherActor :type "Actor Object Reference") (OtherComp :type "PrimitiveComponent Object Reference") (OtherBodyIndex :type Integer))
  (bind _ascharacter (cast `Character` OtherActor))
  (bind _returnvalue (`self.GetComponentByClass` _ascharacter "/Game/AnimationEducation/LLSS/Blueprints/BP_LLSS_Comp.BP_LLSS_Comp_C"))
  (`/Engine/EditorBlueprintResources/StandardMacros.IsValid` _returnvalue
    (:`Is Valid`
      (set `/Game/AnimationEducation/LLSS/Blueprints/BP_LLSS_Comp.InVolume` false _returnvalue))))

(event `self.TriggerLeft.OnComponentBeginOverlap`
  (params (OverlappedComponent :type "PrimitiveComponent Object Reference") (OtherActor :type "Actor Object Reference") (OtherComp :type "PrimitiveComponent Object Reference") (OtherBodyIndex :type Integer) (bFromSweep :type Boolean) (SweepResult :type "HitResult Structure (by ref)"))
  (bind _returnvalue (`SceneComponent.K2_GetComponentToWorld` (`self.LeftTarget`)))
  (bind _ascharacter (cast `Character` OtherActor))
  (bind _returnvalue_2 (`self.GetComponentByClass` _ascharacter "/Game/AnimationEducation/LLSS/Blueprints/BP_LLSS_Comp.BP_LLSS_Comp_C"))
  (`/Engine/EditorBlueprintResources/StandardMacros.IsValid` _returnvalue_2
    (:`Is Valid`
      (set `/Game/AnimationEducation/LLSS/Blueprints/BP_LLSS_Comp.VolumeType` "NewEnumerator1" _returnvalue_2)
      (if (and (not (`/Game/AnimationEducation/LLSS/Blueprints/BP_LLSS_Comp.InTransition` _returnvalue_2)) (`|EnumInequality` (`/Game/AnimationEducation/LLSS/Blueprints/BP_LLSS_Comp.MainState` _returnvalue_2) "NewEnumerator1"))
        (bind _output_get (set `/Game/AnimationEducation/LLSS/Blueprints/BP_LLSS_Comp.BedGround` (`self.GroudBed`) _returnvalue_2))
        (set `/Game/AnimationEducation/LLSS/Blueprints/BP_LLSS_Comp.Mirror` true _returnvalue_2)
        (set `/Game/AnimationEducation/LLSS/Blueprints/BP_LLSS_Comp.ObjectTransforms` (`KismetMathLibrary.MakeTransform` (.location _returnvalue) (`KismetMathLibrary.MakeRotator` (.roll (.rotation _returnvalue)) (.pitch (.rotation _returnvalue)) (+ (.yaw (.rotation _returnvalue)) (select `/Game/AnimationEducation/LLSS/AnimPacks/Lay/Blueprints/Enum/Enum_BedGround` _output_get :`NewEnumerator0` 90.0 :`NewEnumerator1` -180.0)))) _returnvalue_2)
        (set `/Game/AnimationEducation/LLSS/Blueprints/BP_LLSS_Comp.InVolume` true _returnvalue_2)
        (set `/Game/AnimationEducation/LLSS/Blueprints/BP_LLSS_Comp.OverlappedBed` self _returnvalue_2)
        (if (`self.ForcedPose`)
          (bind _output_get_2 (set `/Game/AnimationEducation/LLSS/Blueprints/BP_LLSS_Comp.NextLayType` (`self.LayPose`) _returnvalue_2))
          (set `/Game/AnimationEducation/LLSS/Blueprints/BP_LLSS_Comp.LayType` _output_get_2 _returnvalue_2)
          (set `/Game/AnimationEducation/LLSS/Blueprints/BP_LLSS_Comp.OverlappedChair` null _returnvalue_2)
          (set `/Game/AnimationEducation/LLSS/Blueprints/BP_LLSS_Comp.OverlappedWall` null _returnvalue_2)
          (set `/Game/AnimationEducation/LLSS/Blueprints/BP_LLSS_Comp.VolumeType` "NewEnumerator1" _returnvalue_2))))))

(event `self.TriggerLeft.OnComponentEndOverlap`
  (params (OverlappedComponent :type "PrimitiveComponent Object Reference") (OtherActor :type "Actor Object Reference") (OtherComp :type "PrimitiveComponent Object Reference") (OtherBodyIndex :type Integer))
  (bind _ascharacter (cast `Character` OtherActor))
  (bind _returnvalue (`self.GetComponentByClass` _ascharacter "/Game/AnimationEducation/LLSS/Blueprints/BP_LLSS_Comp.BP_LLSS_Comp_C"))
  (`/Engine/EditorBlueprintResources/StandardMacros.IsValid` _returnvalue
    (:`Is Valid`
      (set `/Game/AnimationEducation/LLSS/Blueprints/BP_LLSS_Comp.InVolume` false _returnvalue))))

(fn `UserConstructionScript`
  (bind _textrender (`self.TextRender`))
  (`SceneComponent.SetVisibility` _textrender (`self.ForcedPose`) false)
  (`TextRenderComponent.K2_SetText` _textrender (`KismetTextLibrary.Conv_StringToText` (`KismetStringLibrary.Concat_StrStr` (`|GetEnumeratorNameAsString` (`self.LayPose`)) " No " (`KismetStringLibrary.Conv_IntToString` (`self.PoseNo`)))))
  (`StaticMeshComponent.SetStaticMesh` (`self.Mesh`) (`self.MainMesh`)))