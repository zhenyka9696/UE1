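; LLSS component that drives a character's standing, sitting, leaning and laying states, including poses, mirroring, rolls and actions.
; Inside a volume, it snaps the character to the object transform, disables gravity and collision, and reads pose data from the overlapped bed, wall or chair.
; It swaps the mesh's Anim Blueprint per state, restoring movement on exit.
; Events set sub-states and clamped pose targets, gated by an InTransition lock.
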(event `Stand`
  (set `self.MainState` "NewEnumerator0")
  (set `self.InTransition` false)
  (bind _output_get (set `self.PoseNumber` 0))
  (bind _output_get_2 (set `self.NextPose` _output_get))
  (set `self.PreviousPose` _output_get_2)
  (set `self.CanLook` true)
  (`KismetSystemLibrary.DelayUntilNextTick`)
  (`SkeletalMeshComponent.SetAnimInstanceClass` (`self.CharacterMesh`) "/Game/AnimationEducation/LLSS/AnimationBlueprint/ABP_Stand.ABP_Stand_C"))

(event `ChangeMainPose`
  (params (PoseType :type "/Game/AnimationEducation/LLSS/AnimPacks/Lay/Blueprints/Enum/Enum_MainState Enum" :default "NewEnumerator0"))
  (set `self.PoseType` PoseType))

(event `ChangeLayType`
  (params (NewParam :type "/Game/AnimationEducation/LLSS/AnimPacks/Lay/Blueprints/Enum/Enum_Faceing Enum" :default "NewEnumerator0"))
  (bind _laytype (`self.LayType`))
  ;[1 1 1 1 30] Comment
  (if (not (`self.InTransition`))
    (set `self.PreviousLayType` _laytype)
    (set `self.PreviousPose` 0)
    (switch `/Game/AnimationEducation/LLSS/AnimPacks/Lay/Blueprints/Enum/Enum_MainState` (`self.MainState`)
      (:`NewEnumerator0`
        (set `self.LayType` NewParam))
      (:`NewEnumerator1`
        (set `self.InTransition` true)
        (switch `/Game/AnimationEducation/LLSS/AnimPacks/Lay/Blueprints/Enum/Enum_Faceing` _laytype
          (:`NewEnumerator0`
            (bind _output_get (set `self.LayType` NewParam))
            (switch `/Game/AnimationEducation/LLSS/AnimPacks/Lay/Blueprints/Enum/Enum_Faceing` _output_get
              (:`NewEnumerator0`
                (set `self.MainState` "NewEnumerator1")
                (set `self.InTransition` false :!label _label))
              (:`NewEnumerator1`
                (set `self.RollType` "NewEnumerator0")
                (set `self.MainState` "NewEnumerator4" :!label _label_2))
              (:`NewEnumerator2`
                (set `self.RollType` "NewEnumerator4")
                (goto _label_2))))
          (:`NewEnumerator1`
            (bind _output_get_2 (set `self.LayType` NewParam))
            (switch `/Game/AnimationEducation/LLSS/AnimPacks/Lay/Blueprints/Enum/Enum_Faceing` _output_get_2
              (:`NewEnumerator0`
                (set `self.RollType` "NewEnumerator1")
                (goto _label_2))
              (:`NewEnumerator1`
                (set `self.MainState` "NewEnumerator1")
                (goto _label))
              (:`NewEnumerator2`
                (set `self.RollType` "NewEnumerator5")
                (goto _label_2))))
          (:`NewEnumerator2`
            (bind _output_get_3 (set `self.LayType` NewParam))
            (switch `/Game/AnimationEducation/LLSS/AnimPacks/Lay/Blueprints/Enum/Enum_Faceing` _output_get_3
              (:`NewEnumerator0`
                (set `self.RollType` "NewEnumerator2")
                (goto _label_2))
              (:`NewEnumerator1`
                (set `self.RollType` "NewEnumerator6")
                (goto _label_2))
              (:`NewEnumerator2`
                (set `self.MainState` "NewEnumerator1")
                (goto _label)))))))))

(event `ChangeMainState`
  (params (Character :type "Character Object Reference") (CharacterMovment :type "CharacterMovementComponent Object Reference"))
  (bind _posenumber (`self.PoseNumber`))
  (bind _mesh (`Character.Mesh` Character))
  (bind _capsulecomponent (`Character.CapsuleComponent` Character))
  ;[1 1 1 1 30] Comment
  (if (not (`self.InTransition`))
    (set `self.CharacterMesh` (`Character.Mesh` Character))
    (switch `/Game/AnimationEducation/LLSS/AnimPacks/Lay/Blueprints/Enum/Enum_MainState` (`self.MainState`)
      (:`NewEnumerator0`
        (if (`self.InVolume`)
          (set `self.CanLook` false)
          (set `self.PreviousGravity` (`CharacterMovementComponent.GravityScale` CharacterMovment))
          (set `CharacterMovementComponent.GravityScale` 0.0 CharacterMovment)
          (`CharacterMovementComponent.SetMovementMode` CharacterMovment "MOVE_Flying" 0)
          (`NavMovementComponent.StopActiveMovement` CharacterMovment)
          (`PrimitiveComponent.SetCollisionEnabled` _capsulecomponent "NoCollision")
          (`Actor.K2_SetActorTransform` Character (`self.ObjectTransforms`) false false)
          (`MovementComponent.StopMovementImmediately` CharacterMovment)
          (set `self.Forward` true)
          (switch `/Game/AnimationEducation/LLSS/AnimPacks/Lay/Blueprints/Enum/Enum_MainState` (`self.VolumeType`)
            (:`NewEnumerator1`
              (bind _overlappedbed (`self.OverlappedBed`)
                (:`then`
                  (set `self.PoseNumber` (`/Game/AnimationEducation/LLSS/Blueprints/BP_Bed.PoseNo` _overlappedbed))
                  (set `self.NextState` "NewEnumerator1")
                  (set `self.MainState` "NewEnumerator1")
                  (`SkeletalMeshComponent.SetAnimInstanceClass` _mesh "/Game/AnimationEducation/LLSS/AnimationBlueprint/ABP_Lay.ABP_Lay_C"))
                (:`else`)))
            (:`NewEnumerator2`
              (bind _overlappedwall (`self.OverlappedWall`)
                (:`then`
                  (set `self.PoseNumber` (`/Game/AnimationEducation/LLSS/Blueprints/BP_LeanWall.PoseNo` _overlappedwall))
                  (set `self.NextState` "NewEnumerator2")
                  (set `self.MainState` "NewEnumerator2")
                  (`SkeletalMeshComponent.SetAnimInstanceClass` _mesh "/Game/AnimationEducation/LLSS/AnimationBlueprint/ABP_Lean.ABP_Lean_C"))
                (:`else`)))
            (:`NewEnumerator4`
              (bind _overlappedchair (`self.OverlappedChair`)
                (:`then`
                  (set `self.PoseNumber` (`/Game/AnimationEducation/LLSS/Blueprints/BP_chair.PoseNo` _overlappedchair))
                  (set `self.SitType` (`/Game/AnimationEducation/LLSS/Blueprints/BP_chair.SitType` _overlappedchair))
                  (set `self.NextState` "NewEnumerator4")
                  (set `self.MainState` "NewEnumerator4")
                  (`SkeletalMeshComponent.SetAnimInstanceClass` _mesh "/Game/AnimationEducation/LLSS/AnimationBlueprint/ABP_Sit.ABP_Sit_C"))
                (:`else`))))
          (set `self.InTransition` true)
          (set `self.PreviousPose` _posenumber)
          (set `self.NextPose` _posenumber)))
      (:`NewEnumerator1`
        (set `self.NextState` "NewEnumerator0" :!label _label_3)
        (set `self.CanLook` false)
        (`PrimitiveComponent.SetCollisionEnabled` (`Character.CapsuleComponent` Character) "QueryAndPhysics")
        (set `CharacterMovementComponent.GravityScale` (`self.PreviousGravity`) CharacterMovment)
        (`CharacterMovementComponent.SetMovementMode` CharacterMovment "MOVE_Walking" 0)
        (`PrimitiveComponent.SetCollisionEnabled` _capsulecomponent "QueryAndPhysics")
        (set `self.InTransition` true))
      (:`NewEnumerator2`
        (goto _label_3))
      (:`NewEnumerator4`
        (goto _label_3)))))

(event `ChangePose`
  (params (PoseNumber :type Integer))
  (bind _intransition (`self.InTransition`))
  (bind _laytype (`self.LayType`))
  (bind _returnvalue (!= PoseNumber (`self.PoseNumber`)))
  (if (and _returnvalue (not _intransition))
    (set `self.NextPose` (`KismetMathLibrary.Clamp` (+ PoseNumber (`KismetMathLibrary.SelectInt` 10 0 (`self.Add10`))) 0 (select `/Game/AnimationEducation/LLSS/AnimPacks/Lay/Blueprints/Enum/Enum_MainState` (`self.MainState`) :`NewEnumerator0` 14 :`NewEnumerator1` (select `/Game/AnimationEducation/LLSS/AnimPacks/Lay/Blueprints/Enum/Enum_Faceing` _laytype :`NewEnumerator0` 9 :`NewEnumerator1` 7 :`NewEnumerator2` 9) :`NewEnumerator2` (select `/Game/AnimationEducation/LLSS/AnimPacks/Lay/Blueprints/Enum/Enum_Faceing` _laytype :`NewEnumerator0` 5 :`NewEnumerator1` 2 :`NewEnumerator2` 4) :`NewEnumerator4` (select `/Game/AnimationEducation/LLSS/AnimPacks/Sit/Blueprints/Enum_SitType` (`self.SitType`) :`NewEnumerator0` 14 :`NewEnumerator1` 11 :`NewEnumerator2` 4))))
    (set `self.SubState` "NewEnumerator5")
    (set `self.InTransition` true)
    (else
      (`KismetSystemLibrary.Delay` 3.0)
      (if (and _returnvalue _intransition)
        (set `self.InTransition` false)
        (set `self.SubState` "NewEnumerator0")))))

(event `MirrorPose`
  (bind _intransition (`self.InTransition`))
  (if (and (not _intransition) (`|EnumInequality` (`self.MainState`) "NewEnumerator2"))
    (set `self.SubState` "NewEnumerator7")
    (set `self.InTransition` true)
    (`KismetSystemLibrary.Delay` 0.2)
    (bind _output_get (set `self.Mirror` (select `bool` (stale _output_get) :`false` true)))
    (set `self.SubState` "NewEnumerator0")
    (else
      (`KismetSystemLibrary.Delay` 3.0)
      (if _intransition
        (set `self.InTransition` false)
        (set `self.SubState` "NewEnumerator0")))))

(event `Roll`
  (params (LayType :type "/Game/AnimationEducation/LLSS/AnimPacks/Lay/Blueprints/Enum/Enum_Faceing Enum" :default "NewEnumerator0"))
  (if (and (not (`self.InTransition`)) (`|EnumEquality` (`self.MainState`) "NewEnumerator1") (`|EnumInequality` LayType (`self.LayType`)))
    (set `self.InTransition` true)
    (bind _output_get (set `self.NextLayType` LayType))
    (set `self.RollType` (select `/Game/AnimationEducation/LLSS/AnimPacks/Lay/Blueprints/Enum/Enum_Faceing` (`self.LayType`) :`NewEnumerator0` (select `/Game/AnimationEducation/LLSS/AnimPacks/Lay/Blueprints/Enum/Enum_Faceing` _output_get :`NewEnumerator0` "NewEnumerator0" :`NewEnumerator1` "NewEnumerator0" :`NewEnumerator2` "NewEnumerator4" :!type "/Game/AnimationEducation/LLSS/AnimPacks/Lay/Blueprints/Enum/Enum_RollType Enum") :`NewEnumerator1` (select `/Game/AnimationEducation/LLSS/AnimPacks/Lay/Blueprints/Enum/Enum_Faceing` _output_get :`NewEnumerator0` "NewEnumerator1" :`NewEnumerator1` "NewEnumerator5" :`NewEnumerator2` "NewEnumerator4" :!type "/Game/AnimationEducation/LLSS/AnimPacks/Lay/Blueprints/Enum/Enum_RollType Enum") :`NewEnumerator2` (select `/Game/AnimationEducation/LLSS/AnimPacks/Lay/Blueprints/Enum/Enum_Faceing` _output_get :`NewEnumerator0` "NewEnumerator2" :`NewEnumerator1` "NewEnumerator6" :`NewEnumerator2` "NewEnumerator4" :!type "/Game/AnimationEducation/LLSS/AnimPacks/Lay/Blueprints/Enum/Enum_RollType Enum")))
    (set `self.SubState` "NewEnumerator6")
    (set `self.NextPose` 0)))

(event `SetAction`
  (params (Action :type "/Game/AnimationEducation/LLSS/Blueprints/Enum/Enum_Action Enum" :default "NewEnumerator0") (EndAction :type Boolean))
  (if (not (`self.InTransition`))
    (set `self.SubState` (select `bool` EndAction :`false` "NewEnumerator4" :`true` "NewEnumerator0" :!type "/Game/AnimationEducation/LLSS/AnimPacks/Sit/Blueprints/Enum_SubStates Enum"))
    (set `self.Action` Action)))