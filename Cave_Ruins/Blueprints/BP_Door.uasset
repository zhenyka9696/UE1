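; Lockable sliding door that the player opens by interacting and that closes when the player leaves its overlap.
; A timeline slides the cube sideways, reversing to close.
; Trigger events unlock keyless doors or lock and close any door, with a point light colored by lock state.
; With RequiredKey set, interacting only unlocks after an inventory check; opening requires that reference to be empty, which DestroyKeyOnUnlock handles by clearing it.
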(event `self.ReceiveActorBeginOverlap`
  (params (OtherActor :type "Actor Object Reference")))

(event `self.ReceiveActorEndOverlap`
  (params (OtherActor :type "Actor Object Reference"))
  (if (== OtherActor (`GameplayStatics.GetPlayerCharacter` 0))
    (`self.CloseDoor`)))

(event `OpenDoor`
  (if (not (`self.IsLocked`))
    (bind (_direction _position) (`Timeline|DoorOpening` :!label _label)
      (:`Update`
        (`SceneComponent.K2_SetRelativeLocation` (`self.Cube`) (* (0.0 250.0 0.0) _position) false false)))))

(event `CloseDoor`
  (goto _label :!via `Reverse`))

(event `self.Trigger.OnTriggered`
  (params (IsTriggered :type Boolean))
  (if IsTriggered
    (`self.RequiredKey`
      (:`then`)
      (:`else`
        (`self.UnlockDoor`)))
    (else
      (`self.LockDoor`))))

(event `/Game/Cave_Ruins/Interfaces/BP_Interact.InteractWith`
  (params (PlayerCharacter :type "/Game/FirstPerson/Blueprints/BP_FirstPersonCharacter Object Reference"))
  (bind _requiredkey (`self.RequiredKey`)
    (:`then`
      (bind _return (`/Game/Game/InventorySystem/InventorySystem.QueryInventory` (`/Game/FirstPerson/Blueprints/BP_FirstPersonCharacter.InventorySystem` PlayerCharacter) _requiredkey 1))
      (if _return
        (`self.UnlockDoor`)))
    (:`else`
      (`self.OpenDoor`))))

(fn `LockDoor`
  (bind _output_get (set `self.IsLocked` true))
  (`LightComponent.SetLightColor` (`self.PointLight`) (`KismetMathLibrary.SelectColor` (struct :`R` 1.0 :`G` 0.319403 :`B` 0.827037 :`A` 1.0) (struct :`R` 0.249227 :`G` 1.0 :`B` 0.228177 :`A` 1.0) _output_get) true)
  (`self.CloseDoor`))

(fn `LookAt`
  (returns (Verb :type Text) (Noun :type Text))
  (return "Open" "door"))

(fn `UnlockDoor`
  (bind _output_get (set `self.IsLocked` false))
  (`LightComponent.SetLightColor` (`self.PointLight`) (`KismetMathLibrary.SelectColor` (struct :`R` 1.0 :`G` 0.319403 :`B` 0.827037 :`A` 1.0) (struct :`R` 0.249227 :`G` 1.0 :`B` 0.228177 :`A` 1.0) _output_get) true)
  (`self.RequiredKey`
    (:`then`
      (if (`self.DestroyKeyOnUnlock`)
        (set `self.RequiredKey` null)))
    (:`else`)))

(fn `UserConstructionScript`
  (`LightComponent.SetLightColor` (`self.PointLight`) (`KismetMathLibrary.SelectColor` (struct :`R` 1.0 :`G` 0.319403 :`B` 0.827037 :`A` 1.0) (struct :`R` 0.249227 :`G` 1.0 :`B` 0.228177 :`A` 1.0) (`self.IsLocked`)) true))