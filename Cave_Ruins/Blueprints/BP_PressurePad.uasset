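; BP_PressurePad is a pressure pad in Cave_Ruins that reacts to the player character stepping on and off it.
; Overlap begin broadcasts OnTriggered as true and lowers the Cube mesh slightly.
; Overlap end raises the Cube immediately and starts a configurable timer, with Timeout available to broadcast OnTriggered as false for a delayed release.
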(event `self.ReceiveActorBeginOverlap`
  (params (OtherActor :type "Actor Object Reference"))
  (if (== OtherActor (`GameplayStatics.GetPlayerCharacter` 0))
    (`self.ButtonTriggered`)))

(event `self.ReceiveActorEndOverlap`
  (params (OtherActor :type "Actor Object Reference"))
  (if (== OtherActor (`GameplayStatics.GetPlayerCharacter` 0))
    (`self.ButtonUntriggered`)))

(event `ButtonTriggered`
  (`self.OnTriggered` true)
  (`SceneComponent.K2_SetRelativeLocation` (`self.Cube`) (0.0 0.0 -10.0) false false))

(event `ButtonUntriggered`
  (`SceneComponent.K2_SetRelativeLocation` (`self.Cube`) (0.0 0.0 0.0) false false)
  (`KismetSystemLibrary.K2_SetTimerDelegate` (`|CreateDelegate` :!event `Timeout`) (`self.Time`)))

(fn `Timeout`
  (`self.OnTriggered` false))

(fn `UserConstructionScript`)